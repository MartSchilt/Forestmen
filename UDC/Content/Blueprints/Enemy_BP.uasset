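; Enemy Blueprint that chases a seen player, takes damage and carries a health bar widget bound to itself on BeginPlay.
; PawnSensing triggers AI MoveTo toward the player, while Hit passes damage to TakeDamage and updates animation state.
; DisplayHPBar shows the bar; Tick hides it beyond the Paladin's detection range plus an offset.
; Kill decrements the TimeActor count and opens MainMenu once it reaches zero.
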(event OnSeePawn(PawnSensing)
  (params (Pawn :type Pawn%20Object%20Reference))
  ;[1 1 1] Move to the Player
  (bind _asplayer_character (Utilities|Casting|CastToPlayerCharacter Pawn))
  (AI|AIMoveTo self "0, 0, 0" _asplayer_character 5.0 false))

(event Custom|Hit
  (params (Damage :type Float%20%28single-precision%29))
  ;[1 1 1] Taking Damage
  (bind _returnvalue (Class|NonPlayablaCharacter|TakeDamage Damage))
  (Variables|Default|SetPlayAnimation _returnvalue)
  (Variables|Default|SetDead (Variables|Default|GetbDead)))

(event Custom|Kill
  ;[1 1 1] Death Handling
  (bind _returnvalue (Actor|GetActorOfClass "/Script/UDC.TimeActor"))
  (bind _astime_actor (Utilities|Casting|CastToTimeActor _returnvalue))
  (Class|TimeActor|Decrease _astime_actor)
  (if (<= (Variables|/Script/UDC.TimeActor|GetCount _astime_actor) 0)
    (Actor|GetActorOfClass "/Game/Blueprints/PlayerCharacter_Paladin.PlayerCharacter_Paladin_C")
    (Game|OpenLevel(byName) "MainMenu")))

(event EventBeginPlay
  ;[1 1 1] Set the HenkPoints UI
  (bind _asenemy_henk_points_ui (Utilities|Casting|CastToEnemyHenkPointsUI (UserInterface|GetUserWidgetObject (Variables|Default|GetEnemyHenkPointsUI))))
  (Variables|/Game/UI/EnemyHenkPointsUI.EnemyHenkPointsUI_C|SetEnemy _asenemy_henk_points_ui self))

(event EventTick
  (params (DeltaSeconds :type Float%20%28single-precision%29))
  (bind _returnvalue (Game|GetPlayerCharacter 0))
  ;[1 1 1] Visibility HP Bar
  (bind _asplayer_character_paladin (Utilities|Casting|CastToPlayerCharacter_Paladin _returnvalue))
  (if (and (Rendering|IsVisible (Variables|Default|GetEnemyHenkPointsUI)) (> (Transformation|GetDistanceTo _returnvalue) (+ (Variables|/Game/Blueprints/PlayerCharacter_Paladin.PlayerCharacter_Paladin_C|GetEnemyDetectionRange _asplayer_character_paladin) (Variables|Default|GetOffsetDetectionRange))))
    (Rendering|SetVisibility (Variables|Default|GetEnemyHenkPointsUI) false false)))

(fn ConstructionScript)

(fn DisplayHPBar
  (Rendering|SetVisibility (Variables|Default|GetEnemyHenkPointsUI) true false))