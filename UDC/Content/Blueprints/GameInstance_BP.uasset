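; Game instance that holds audio volume settings and run state: primary and secondary type and rarity, plus a count of levels cleared.
; UpdateAudio applies the stored master, music and sound effects volumes as sound class overrides on a shared sound mix.
; Reset returns both slots to Common rarity with their default types and zeroes the cleared-level count.
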(fn UpdateAudio
  (Audio|SetSoundMixClassOverride "/Game/Audio/AudioMix.AudioMix" "/Game/Audio/AudioMaster.AudioMaster" (Variables|Default|GetAudioMaster) 1.0 1.0 true)
  (Audio|SetSoundMixClassOverride "/Game/Audio/AudioMix.AudioMix" "/Game/Audio/Music.Music" (Variables|Default|GetAudioMusic) 1.0 1.0 true)
  (Audio|SetSoundMixClassOverride "/Game/Audio/AudioMix.AudioMix" "/Game/Audio/SoundFX.SoundFX" (Variables|Default|GetAudioSoundFX) 1.0 1.0 true))

(fn Reset
  (Variables|Default|SetPrimaryRarity "Common")
  (Variables|Default|SetPrimaryType "NewEnumerator0")
  (Variables|Default|SetSecondaryRarity "Common")
  (Variables|Default|SetSecondaryType "NewEnumerator1")
  (Variables|Default|SetLevelsCleared 0))