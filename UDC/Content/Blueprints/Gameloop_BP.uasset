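; Game loop Blueprint that runs a countdown and reports win or loss from the remaining enemy count.
; Tick drives the clock through a one-second Delay while EnemyCount is above zero, decrementing Seconds and rolling over into Minutes.
; Reaching 0:00 prints a loss message, while a Tick with no enemies left prints a win message.
; Results are only printed strings, and EnemyCount is never changed in this graph.
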(event EventBeginPlay)

(event EventTick
  (params (DeltaSeconds :type Float%20%28single-precision%29))
  (if (> (Variables|Default|GetEnemyCount) 0)
    (Utilities|FlowControl|Delay 1.0)
    (Variables|Default|SetSeconds (- (Variables|Default|GetSeconds) 1))
    (if (< (Variables|Default|GetSeconds) 0)
      (Variables|Default|SetMinutes (- (Variables|Default|GetMinutes) 1))
      (Variables|Default|SetSeconds 59))
    (if (== (Variables|Default|GetSeconds) 0)
      (if (== (Variables|Default|GetMinutes) 0)
        (if (not (< (Variables|Default|GetEnemyCount) 0))
          (Development|PrintString "Moron you lost"))))
    (else
      (Development|PrintString "Good Job you won"))))

(event Collision|EventActorBeginOverlap
  (params (OtherActor :type Actor%20Object%20Reference)))

(fn ConstructionScript)