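; PlayerCharacter_GameMode_BP is a game mode Blueprint that ends the match in defeat when time runs out.
; Each Tick it finds the TimeActor in the level and checks whether both its Minutes and Seconds equal -1.
; When they do, it sets Victory to false on GameInstance_BP and opens the MainMenu level.
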(event EventBeginPlay)

(event EventTick
  (params (DeltaSeconds :type Float%20%28single-precision%29))
  (bind _returnvalue (Actor|GetActorOfClass "/Script/UDC.TimeActor"))
  (bind _astime_actor (Utilities|Casting|CastToTimeActor _returnvalue))
  (if (== (Variables|/Script/UDC.TimeActor|GetMinutes _astime_actor) -1)
    (if (== (Variables|/Script/UDC.TimeActor|GetSeconds _astime_actor) -1)
      (bind _asgame_instance_bp (Utilities|Casting|CastToGameInstance_BP (Game|GetGameInstance)))
      (Variables|/Game/Blueprints/GameInstance_BP.GameInstance_BP_C|SetVictory _asgame_instance_bp false)
      (Game|OpenLevel(byName) "MainMenu"))))

(fn ConstructionScript)