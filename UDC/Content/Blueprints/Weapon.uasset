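; Weapon actor that the player picks up from the world and uses to damage enemies.
; A Dropped/Equipped state toggles mesh physics and collision, with a rotation fix for swords.
; While unequipped, interaction range shows a screen-space "Pick Up" widget component created at runtime, and interacting hands the weapon to the player.
; Box overlaps during the Paladin player's attack pass rarity-based damage to the enemy's Die function.
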(event OnComponentBeginOverlap(Box)
  (params (OverlappedComponent :type Primitive%20Component%20Object%20Reference) (OtherActor :type Actor%20Object%20Reference) (OtherComp :type Primitive%20Component%20Object%20Reference) (OtherBodyIndex :type Integer) (bFromSweep :type Boolean) (SweepResult :type Hit%20Result%20Structure%20%28by%20ref%29))
  ;[1 1 1] Attack Damage
  (bind _asplayer_character_paladin (Utilities|Casting|CastToPlayerCharacter_Paladin (Game|GetPlayerCharacter 0)))
  (if (Variables|/Game/Blueprints/PlayerCharacter_Paladin.PlayerCharacter_Paladin_C|GetAttack _asplayer_character_paladin)
    (bind _asenemy_bp (Utilities|Casting|CastToEnemy_BP OtherActor))
    (bind _returnvalue (Class|Sword|GetDamage (Variables|Default|GetRarity)))
    (Default|Die _asenemy_bp _returnvalue)))

(event OnComponentBeginOverlap(Sphere)
  (params (OverlappedComponent :type Primitive%20Component%20Object%20Reference) (OtherActor :type Actor%20Object%20Reference) (OtherComp :type Primitive%20Component%20Object%20Reference) (OtherBodyIndex :type Integer) (bFromSweep :type Boolean) (SweepResult :type Hit%20Result%20Structure%20%28by%20ref%29))
  (Variables|Default|SetOverlap true))

(event OnComponentEndOverlap(Sphere)
  (params (OverlappedComponent :type Primitive%20Component%20Object%20Reference) (OtherActor :type Actor%20Object%20Reference) (OtherComp :type Primitive%20Component%20Object%20Reference) (OtherBodyIndex :type Integer))
  (Variables|Default|SetOverlap false))

(event EventBeginPlay
  (CallFunction|SetWeaponState "NewEnumerator0"))

(event EventTick
  (params (DeltaSeconds :type Float%20%28single-precision%29))
  (if (Variables|Default|GetIsEquipped)
    (bind _interactionwidgetcomponent (Variables|Default|GetInteractionWidgetComponent)
      (:then
        (Components|DestroyComponent _interactionwidgetcomponent))
      (:else))))

(event EventOnInteractionRangeEntered
  (params (Player :type Player%20Character%20Paladin%20Object%20Reference))
  (if (not (Variables|Default|GetIsEquipped))
    (Variables|Default|GetInteractionWidgetComponent
      (:then)
      (:else
        (bind _returnvalue (UserInterface|CreateWidget "/Game/InteractionInterface/InteractionWidget.InteractionWidget_C" (.AsPlayer%20Controller (Utilities|Casting|CastToPlayerController (Pawn|GetController Player))) (CallFunction|GetInteractionText)))
        (bind _returnvalue_2 (AddComponent|AddWidgetComponent false))
        (bind _output_get (Variables|Default|SetInteractionWidgetComponent _returnvalue_2))
        (UserInterface|SetWidget _output_get _returnvalue)
        (Utilities|FlowControl|Sequence
          (:then_0
            (Class|WidgetComponent|SetWidgetSpace _output_get "Screen"))
          (:then_1
            (Class|WidgetComponent|SetDrawatDesiredSize _output_get true))
          (:then_2
            (Collision|SetCollisionEnabled _output_get "NoCollision"))
          (:then_3
            (Transformation|AttachComponentToComponent _output_get (CallFunction|GetInteractionTextAttach) "None" "SnapToTarget" "SnapToTarget" "SnapToTarget" true)))))))

(event EventOnInteractionRangeExited
  (if (not (Variables|Default|GetIsEquipped))
    (bind _interactionwidgetcomponent (Variables|Default|GetInteractionWidgetComponent)
      (:then
        (Components|DestroyComponent _interactionwidgetcomponent))
      (:else))))

(event EventOnInteracted
  (params (Player :type Player%20Character%20Paladin%20Object%20Reference))
  (if (not (Variables|Default|GetIsEquipped))
    (Default|PickUpWeapon Player self)
    (CallFunction|SetWeaponState "NewEnumerator1")))

(fn ConstructionScript)

(fn SetWeaponState
  (params (NewWeaponState :type EnumState%20Enum :default "NewEnumerator0"))
  (bind _skeletalmesh (Variables|Default|GetSkeletalMesh))
  (bind _skeletalmesh_2 (Variables|Default|GetSkeletalMesh))
  (bind _output_get (Variables|Default|SetWeaponState NewWeaponState))
  (switch Utilities|FlowControl|Switch|SwitchonEnumState _output_get
    (:NewEnumerator0
      (Collision|SetCollisionProfileName (Variables|Default|GetSphere) "OverlapAllDynamic" :!class /Script/Engine.PrimitiveComponent)
      (Physics|SetSimulatePhysics _skeletalmesh true)
      (Collision|SetCollisionProfileName _skeletalmesh "DroppedWeapon" :!class /Script/Engine.PrimitiveComponent))
    (:NewEnumerator1
      (Collision|SetCollisionProfileName (Variables|Default|GetSphere) "NoCollision" :!class /Script/Engine.PrimitiveComponent)
      (Physics|SetSimulatePhysics _skeletalmesh_2 false)
      (Collision|SetCollisionProfileName _skeletalmesh_2 "NoCollision" :!class /Script/Engine.PrimitiveComponent)
      (Transformation|ResetRelativeTransform _skeletalmesh_2)
      (switch Utilities|FlowControl|Switch|SwitchonEnumType (Variables|Default|GetWeaponType)
        (:NewEnumerator0
          (Transformation|SetActorRelativeRotation "-180.000000, 0, 0"))))))

(fn GetInteractionTextAttach
  (return (Variables|Default|GetSkeletalMesh)))

(fn Drop
  (CallFunction|SetWeaponState "NewEnumerator0")
  (Variables|Default|SetIsEquipped false))

(fn GetInteractionText
  (return "Pick Up"))