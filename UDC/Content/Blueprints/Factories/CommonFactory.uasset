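; CommonFactory is a weapon factory Blueprint that spawns Common rarity weapons.
; CreateAxe, CreateSpear and CreateSword each spawn an actor at the Location variable, then set its Rarity to Common.
; All three events spawn the Weapon_Axe class, so the spear and sword events also produce axes.
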(event EventCreateAxe
  (bind _returnvalue (Game|SpawnActorfromClass "/Game/Blueprints/Weapon_Axe.Weapon_Axe_C" (Math|Transform|MakeTransform (Variables|Default|GetLocation) "0, 0, 0" "1,1,1") "Undefined" 0 0))
  (Variables|/Game/Blueprints/Weapon.Weapon_C|SetRarity _returnvalue "Common"))

(event EventCreateSpear
  (bind _returnvalue (Game|SpawnActorfromClass "/Game/Blueprints/Weapon_Axe.Weapon_Axe_C" (Math|Transform|MakeTransform (Variables|Default|GetLocation) "0, 0, 0" "1,1,1") "Undefined" 0 0))
  (Variables|/Game/Blueprints/Weapon.Weapon_C|SetRarity _returnvalue "Common"))

(event EventCreateSword
  (bind _returnvalue (Game|SpawnActorfromClass "/Game/Blueprints/Weapon_Axe.Weapon_Axe_C" (Math|Transform|MakeTransform (Variables|Default|GetLocation) "0, 0, 0" "1,1,1") "Undefined" 0 0))
  (Variables|/Game/Blueprints/Weapon.Weapon_C|SetRarity _returnvalue "Common"))

(fn ConstructionScript)