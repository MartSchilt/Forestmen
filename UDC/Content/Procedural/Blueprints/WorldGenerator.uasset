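; Procedural level builder that turns the WorldGenerator's rooms and corridors into a playable layout at BeginPlay.
; Each room streams a random level instance from a data table, and square perimeter walls are built from instanced meshes around room centres.
; Corridors are instanced meshes interpolated along each segment and drawn as debug lines every Tick.
; With a valid player, it teleports them to the first room and spawns a ChargerCommon enemy in every room.
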(event EventBeginPlay
  (bind _returnvalue (Game|GetPlayerCharacter 0))
  (bind _worldgenerator (Variables|Actor|GetWorldGenerator))
  (Class|WorldGenerator|SpawnRooms _worldgenerator)
  (for _array_element (Variables|/Script/UDC.WorldGenerator|Getrooms _worldgenerator)
    (Utilities|Array|Add (Variables|Default|GetRoomPositions) (* (.roomposition _array_element) (Variables|/Script/UDC.WorldGenerator|GettileSize (Variables|Actor|GetWorldGenerator))))
    (CallFunction|SpawnRandomRoom (* (.roomposition _array_element) (Variables|/Script/UDC.WorldGenerator|GettileSize (Variables|Actor|GetWorldGenerator))))
    (CallFunction|SpawnRoomWalls))
  (CallFunction|SpawnCorridors)
  (Utilities|IsValid _returnvalue
    (:Is%20Valid
      (Transformation|SetActorLocation _returnvalue (+ (* (Utilities|Struct|BreakRoomStruct (Utilities|Array|Get(acopy) (Variables|/Script/UDC.WorldGenerator|Getrooms (Variables|Actor|GetWorldGenerator)))) 1e+02) "0, 0,200.000000") false true)
      (CallFunction|SpawnEnemies))))

(event EventTick
  (params (DeltaSeconds :type Float%20%28single-precision%29))
  (for _array_element (Variables|/Script/UDC.WorldGenerator|Getcorridors (Variables|Actor|GetWorldGenerator))
    (Rendering|Debug|DrawDebugLine (* (.from (Utilities|Struct|BreakCorridorStruct _array_element)) 100) (* (.to (Utilities|Struct|BreakCorridorStruct _array_element)) 100) "(R=0.024782,G=0.000000,B=0.468750,A=1.000000)" 0.0 1e+02)))

(fn ConstructionScript)

(fn SpawnRandomRoom
  (params (Location :type Vector))
  (LocalVariables|Setposition Location)
  (bind _outrownames (DataTable|GetDataTableRowNames (Variables|Default|GetDataTableRooms)))
  (bind _returnvalue (Utilities|GetDataTableRow (Variables|Default|GetDataTableRooms) (Utilities|Array|Get(acopy) _outrownames (Math|Random|RandomInteger (Utilities|Array|Length _outrownames))))
    (:then
      (Class|LevelStreamingDynamic|LoadLevelInstance (Utilities|Struct|BreakLevelData (Utilities|Struct|BreakLevelEntry _returnvalue)) (LocalVariables|Getposition) "0, 0, 0"))))

(fn SpawnCorridors
  (for _array_element (Variables|/Script/UDC.WorldGenerator|Getcorridors (Variables|Actor|GetWorldGenerator))
    (bind _output_get (LocalVariables|SetFrom (* (.from _array_element) 100)))
    (bind _output_get_2 (LocalVariables|SetTo (* (.to _array_element) 100)))
    (bind _output_get_3 (LocalVariables|SetobjectsToCreate (/ (Math|Vector|Distance(Vector) _output_get _output_get_2) 1e+02)))
    (LocalVariables|SetDistance (/ 1.0 _output_get_3))
    (for _index (range 0 (Math|Float|Truncate _output_get_3))
      (Components|InstancedStaticMesh|AddInstance (Variables|Default|GetCorridor) (Math|Transform|MakeTransform (+ (Math|Vector|Lerp(Vector) (LocalVariables|GetFrom) (LocalVariables|GetTo) (LocalVariables|GetLerpValue)) "50.000000,50.000000,-1.000000")))
      (LocalVariables|SetLerpValue (+ (LocalVariables|GetDistance) (LocalVariables|GetLerpValue))))
    (LocalVariables|SetLerpValue 0.0)))

(fn SpawnEnemies
  (for _array_element (Variables|/Script/UDC.WorldGenerator|Getrooms (Variables|Actor|GetWorldGenerator))
    (bind _returnvalue (Game|SpawnActorfromClass "/Game/Blueprints/Enemies/ChargerCommon.ChargerCommon_C" (Math|Conversions|ToTransform(Vector) (+ (* (.roomCenter (Utilities|Struct|BreakRoomStruct _array_element)) 100) "0.000000, 0,200.000000" "")) "AdjustIfPossibleButAlwaysSpawn" 0 0))
    (Pawn|SpawnDefaultController _returnvalue)))

(fn SpawnRoomWalls
  (CallFunction|CalculateRoomPoints)
  (for _array_element (Variables|Default|GetPoints)
    (CallFunction|CreateWall (.v1 _array_element) (.v2 _array_element))))

(fn CreateWall
  (params (StartPoint :type Vector) (EndPoint :type Vector))
  (bind _returnvalue (Math|Rotator|FindLookatRotation StartPoint EndPoint))
  (bind _returnvalue_2 (Math|Rotator|MakeRotator 0.0 0.0 (.yaw _returnvalue)))
  (Components|StaticMesh|SetStaticMesh (Variables|Default|GetWall) "/Game/StarterContent/Architecture/Wall_400x400.Wall_400x400")
  (bind _output_get (LocalVariables|SetVectorLengthTemp (Math|Vector|Distance(Vector) StartPoint (* EndPoint "1.000000,1.000000, 0"))))
  (if (> (- (Math|Float|Round (/ _output_get (Variables|Default|GetMeshLength))) 1) 0)
    (for _index (range 0 (- (Math|Float|Round (/ _output_get (Variables|Default|GetMeshLength))) 1))
      (Components|InstancedStaticMesh|AddInstance (Variables|Default|GetWall) (Math|Transform|MakeTransform (+ StartPoint (Math|Vector|RotateVector (Math|Vector|MakeVector (- (LocalVariables|GetVectorLengthTemp) (- (LocalVariables|GetVectorLengthTemp) (* _index (Variables|Default|GetMeshLength)))) 0.0 0.0) _returnvalue_2)) _returnvalue_2 "0.250000,1.000000,1.000000")))))

(fn CalculateRoomPoints
  (bind _points (Variables|Default|GetPoints))
  (for _array_element (Variables|/Script/UDC.WorldGenerator|Getrooms (Variables|Actor|GetWorldGenerator))
    (for _index (range 0 3)
      (switch int _index
        (:0
          (Utilities|Array|Add _points (Utilities|Struct|MakeTwoVectors (Math|Vector|MakeVector (- (.x (* (Utilities|Struct|BreakRoomStruct _array_element) (Variables|/Script/UDC.WorldGenerator|GettileSize (Variables|Actor|GetWorldGenerator)))) 2.5e+03) (+ (.y (* (Utilities|Struct|BreakRoomStruct _array_element) (Variables|/Script/UDC.WorldGenerator|GettileSize (Variables|Actor|GetWorldGenerator)))) 2.5e+03) 0.0) (Math|Vector|MakeVector (+ (.x (* (Utilities|Struct|BreakRoomStruct _array_element) (Variables|/Script/UDC.WorldGenerator|GettileSize (Variables|Actor|GetWorldGenerator)))) 2.5e+03) (+ (.y (* (Utilities|Struct|BreakRoomStruct _array_element) (Variables|/Script/UDC.WorldGenerator|GettileSize (Variables|Actor|GetWorldGenerator)))) 2.5e+03) 0.0))))
        (:1
          (Utilities|Array|Add _points (Utilities|Struct|MakeTwoVectors (Math|Vector|MakeVector (+ (.x (* (Utilities|Struct|BreakRoomStruct _array_element) (Variables|/Script/UDC.WorldGenerator|GettileSize (Variables|Actor|GetWorldGenerator)))) 2.5e+03) (+ (.y (* (Utilities|Struct|BreakRoomStruct _array_element) (Variables|/Script/UDC.WorldGenerator|GettileSize (Variables|Actor|GetWorldGenerator)))) 2.5e+03) 0.0) (Math|Vector|MakeVector (+ (.x (* (Utilities|Struct|BreakRoomStruct _array_element) (Variables|/Script/UDC.WorldGenerator|GettileSize (Variables|Actor|GetWorldGenerator)))) 2.5e+03) (- (.y (* (Utilities|Struct|BreakRoomStruct _array_element) (Variables|/Script/UDC.WorldGenerator|GettileSize (Variables|Actor|GetWorldGenerator)))) 2.5e+03) 0.0))))
        (:2
          (Utilities|Array|Add _points (Utilities|Struct|MakeTwoVectors (Math|Vector|MakeVector (+ (.x (* (Utilities|Struct|BreakRoomStruct _array_element) (Variables|/Script/UDC.WorldGenerator|GettileSize (Variables|Actor|GetWorldGenerator)))) 2.5e+03) (- (.y (* (Utilities|Struct|BreakRoomStruct _array_element) (Variables|/Script/UDC.WorldGenerator|GettileSize (Variables|Actor|GetWorldGenerator)))) 2.5e+03) 0.0) (Math|Vector|MakeVector (- (.x (* (Utilities|Struct|BreakRoomStruct _array_element) (Variables|/Script/UDC.WorldGenerator|GettileSize (Variables|Actor|GetWorldGenerator)))) 2.5e+03) (- (.y (* (Utilities|Struct|BreakRoomStruct _array_element) (Variables|/Script/UDC.WorldGenerator|GettileSize (Variables|Actor|GetWorldGenerator)))) 2.5e+03) 0.0))))
        (:3
          (Utilities|Array|Add _points (Utilities|Struct|MakeTwoVectors (Math|Vector|MakeVector (- (.x (* (Utilities|Struct|BreakRoomStruct _array_element) (Variables|/Script/UDC.WorldGenerator|GettileSize (Variables|Actor|GetWorldGenerator)))) 2.5e+03) (- (.y (* (Utilities|Struct|BreakRoomStruct _array_element) (Variables|/Script/UDC.WorldGenerator|GettileSize (Variables|Actor|GetWorldGenerator)))) 2.5e+03) 0.0) (Math|Vector|MakeVector (- (.x (* (Utilities|Struct|BreakRoomStruct _array_element) (Variables|/Script/UDC.WorldGenerator|GettileSize (Variables|Actor|GetWorldGenerator)))) 2.5e+03) (+ (.y (* (Utilities|Struct|BreakRoomStruct _array_element) (Variables|/Script/UDC.WorldGenerator|GettileSize (Variables|Actor|GetWorldGenerator)))) 2.5e+03) 0.0))))))))