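; DungeonGenerator is an actor Blueprint that builds a random dungeon at BeginPlay using RoomGenerator.
; It places rooms until too many tries fail, then streams a random DungeonRooms data table level instance, unrotated, at each scaled room position.
; It then calls CreateSpanningTreeV2, and Tick draws the generator's corridors as debug lines.
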(event EventBeginPlay
  (bind _roomgenerator (Variables|Default|GetRoomGenerator))
  (bind _roomsize (Variables|/Script/UDC.RoomGenerator|GetroomSize _roomgenerator))
  (while (not (Class|RoomGenerator|TooManyTries (Variables|Default|GetRoomGenerator)))
    (Class|RoomGenerator|TryPlaceRoom (Variables|Default|GetRoomGenerator)))
  (for (_array_element _array_index) (Variables|/Script/UDC.RoomGenerator|GetroomsData (Variables|Default|GetRoomGenerator))
    (Variables|Default|SetCurrentRoom _array_index)
    (bind _outrownames (DataTable|GetDataTableRowNames "/Game/Procedural/DataTable/DungeonRooms.DungeonRooms"))
    (bind _returnvalue (Utilities|GetDataTableRow "/Game/Procedural/DataTable/DungeonRooms.DungeonRooms" (Utilities|Array|Get(acopy) _outrownames (Math|Random|RandomInteger (Utilities|Array|Length _outrownames))))
      (:then
        (bind _returnvalue_2 (Class|RoomGenerator|GetRandomRotation (Variables|Default|GetRoomGenerator)))
        (Class|LevelStreamingDynamic|LoadLevelInstance (.Map (Utilities|Struct|BreakLevelData (Utilities|Struct|BreakLevelEntry _returnvalue))) (Math|Vector|MakeVector (* (.X (Math|Vector|BreakVector (Utilities|Struct|BreakRoomData _array_element))) _roomsize) (* (.Y (Math|Vector|BreakVector (Utilities|Struct|BreakRoomData _array_element))) _roomsize) (* (.Z (Math|Vector|BreakVector (Utilities|Struct|BreakRoomData _array_element))) _roomsize)) "0, 0, 0"))))
  (Class|RoomGenerator|CreateSpanningTreeV2 _roomgenerator))

(event Collision|EventActorBeginOverlap
  (params (OtherActor :type Actor%20Object%20Reference)))

(event EventTick
  (params (DeltaSeconds :type Float%20%28single-precision%29))
  (bind _roomgenerator (Variables|Default|GetRoomGenerator))
  (for _array_element (Variables|/Script/UDC.RoomGenerator|GetCorridors _roomgenerator)
    (Rendering|Debug|DrawDebugLine (* (.from (Utilities|Struct|BreakCorridor _array_element)) 1e+02) (* (.to (Utilities|Struct|BreakCorridor _array_element)) 1e+02) "(R=0.713542,G=0.000000,B=0.459756,A=1.000000)" 0.0 5e+01))
  (for _array_element_2 (Variables|/Script/UDC.RoomGenerator|GetroomsData _roomgenerator)
    _))

(fn ConstructionScript)